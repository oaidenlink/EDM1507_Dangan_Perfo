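; BP_ClockManager runs a Quartz musical clock named LebronClock and reports its timing on screen.
; On BeginPlay it creates and stores the clock, applies the BeatsPerMinute tempo, starts it and subscribes to quarter-note quantization events.
; Each quantization event prints the clock, bar and beat as a keyed debug string that replaces the previous one.
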(event `self.ReceiveBeginPlay`
  (bind _returnvalue (`QuartzSubsystem.CreateNewClock` :`self` (subsystem `QuartzSubsystem`) :`ClockName` "LebronClock"))
  ; sauver dans une varable
  (bind _output_get (set `self.LebronClock` _returnvalue))
  ; set le bpm
  (bind _clockhandle (`QuartzClockHandle.SetBeatsPerMinute` :`self` _output_get :`BeatsPerMinute` (`self.Beats Per Minute`)))
  ; commencer le clock
  (bind _clockhandle_2 (`QuartzClockHandle.StartClock` _clockhandle))
  (`QuartzClockHandle.SubscribeToQuantizationEvent` _clockhandle_2 "QuarterNote" (`|CreateDelegate` :!event `QuantizationEvent`)))

(event `QuantizationEvent`
  (params (LebronClock :type Name) (QuantizationType :type "EQuartzCommandQuantization Enum" :default "Bar") (NumBars :type Integer) (Beat :type Integer) (BeatFraction :type "Float (single-precision)"))
  (`KismetSystemLibrary.PrintString` (`KismetTextLibrary.Conv_TextToString` (`|FormatText` "{clock} {bar} {beat}" LebronClock NumBars Beat)) true true (struct :`G` 0.66 :`B` 1.0 :`A` 1.0) 1.0 "clock"))

(fn `UserConstructionScript`)